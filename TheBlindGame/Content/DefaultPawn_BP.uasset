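; Default pawn Blueprint that lets the player grab an AI chicken to open a room door.
; BeginPlay finds door and AI pawn actors with nested GetAllActorsOfClass loops, keeping the last of each as its targets.
; The Grabber's OnGrab event stops the stored chicken's movement, opens the stored door, then destroys the chicken after a delay, without checking which object was grabbed.
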(event OnGrab(Grabber)
  ;[1 1 1] Kada uspješno dohvatimo kokoš, onemogućimo joj kretanje i otvorimo vrata prostorije
  (Components|Movement|StopMovementImmediately (Pawn|GetMovementComponent (Variables|Default|GetAIChicken)))
  (Default|OpenDoors (Variables|Default|GetTarget%20Door))
  (Utilities|FlowControl|Delay 5.0)
  (Actor|DestroyActor (Variables|Default|GetAIChicken)))

(event EventBeginPlay
  ;[1 1 1] Moramo specificirati varijable prilikom run-timea s kojima komunicira Default Pawn
  ;;[1 1 1] Odredimo koja vrata želimo otvoriti
  (bind _outactors (Actor|GetAllActorsOfClass "/Game/SM_Door_BP.SM_Door_BP_C"))
  (for _array_element _outactors
    (Variables|Default|SetTarget%20Door _array_element)
    ;;[1 1 1] Odredimo kojem AI želimo onemogućiti kretanje
    (bind _outactors_2 (Actor|GetAllActorsOfClass "/Game/AI/AIPawn_BP.AIPawn_BP_C"))
    (for _array_element_2 _outactors_2
      (Variables|Default|SetAIChicken _array_element_2))))

(fn ConstructionScript)