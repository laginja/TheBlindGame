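; AI pawn Blueprint that wanders between random navigable points, starting at BeginPlay.
; MoveToRandomLocation picks a point within a fixed radius of the pawn and calls itself again after each successful AI MoveTo, with no handling for failed moves.
; A Chase event similarly loops toward the player pawn with a delay between moves, but its only outside call is unreachable, so chasing never starts here.
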(event Custom|MoveToRandomLocation
  (AI|AIMoveTo self (Class|NavigationSystem|GetRandomPointinNavigableRadius (Transformation|GetActorLocation) 5e+02) 0 5.0 false
    (:OnSuccess
      (CallFunction|MovetoRandomLocation))))

(event Custom|Chase
  (AI|AIMoveTo self "0, 0, 0" (Game|Player|GetPlayerPawn 0) 1e+02 false
    (:OnSuccess
      (Utilities|FlowControl|Delay 1.0)
      (CallFunction|Chase))))

(event EventBeginPlay
  (CallFunction|MovetoRandomLocation))

(fn ConstructionScript
  (|CallParentFunction))