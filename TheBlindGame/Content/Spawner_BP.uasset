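; Spawner actor that places the AI_master_BP master AI around the player's pawn when spawn or respawn events fire.
; On BeginPlay it binds handlers to both events.
; Spawning destroys the referenced MasterAI and creates a new one at the FirstSpawn angle, offset by Radius through cosine and sine at pawn height.
; Respawning destroys every AI_master_BP instance and spawns one using random angles with the same radial offset.
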(event Custom|SpawnMaster_Event
  (bind _returnvalue (Game|GetPlayerController 0))
  (bind _firstspawn (Variables|Default|GetFirstSpawn))
  (bind _radius (Variables|Default|GetRadius))
  (bind _returnvalue_2 (Pawn|GetControlledPawn _returnvalue))
  (bind _returnvalue_3 (Transformation|GetActorLocation _returnvalue_2))
  (bind (_x _y _z) (Math|Vector|BreakVector _returnvalue_3))
  (Actor|DestroyActor (Variables|Default|GetMasterAI))
  (Game|SpawnActorfromClass "/Game/AI/AI_master_BP.AI_master_BP_C" (Math|Transform|MakeTransform (Math|Vector|MakeVector (+ _x (* (Math|Trig|Cos(Degrees) _firstspawn) _radius)) (+ _y (* (Math|Trig|Sin(Degrees) _firstspawn) _radius)) _z) "0, 0, 0" "1,1,1") "Undefined" 0 0))

(event Custom|RespawnMaster_Event
  (bind _returnvalue (Game|GetPlayerController 0))
  (bind _returnvalue_2 (Math|Random|RandomFloatinRange 0.0 359.0))
  (bind _radius (Variables|Default|GetRadius))
  (bind _returnvalue_3 (Pawn|GetControlledPawn _returnvalue))
  (bind _returnvalue_4 (Transformation|GetActorLocation _returnvalue_3))
  (bind (_x _y _z) (Math|Vector|BreakVector _returnvalue_4))
  (bind _outactors (Actor|GetAllActorsOfClass "/Game/AI/AI_master_BP.AI_master_BP_C"))
  (Actor|DestroyActor _outactors)
  (Game|SpawnActorfromClass "/Game/AI/AI_master_BP.AI_master_BP_C" (Math|Transform|MakeTransform (Math|Vector|MakeVector (+ _x (* (Math|Trig|Cos(Degrees) _returnvalue_2) _radius)) (+ _y (* (Math|Trig|Sin(Degrees) _returnvalue_2) _radius)) _z) "0, 0, 0" "1,1,1") "Undefined" 0 0))

(event EventBeginPlay
  (EventDispatchers|BindEventtoSpawnMaster (delegate Custom|SpawnMaster_Event))
  (EventDispatchers|BindEventtoRespawnMaster (delegate Custom|RespawnMaster_Event)))

(fn ConstructionScript)